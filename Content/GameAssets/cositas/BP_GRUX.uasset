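; BP_GRUX is a Grux melee enemy that stays still until PawnSensing sees a pawn, then chases the player.
; Each sighting runs AI MoveTo; on arrival it plays an attack montage, damages "player"-tagged actors in a sphere at an arrow, and waits out the montage.
; AnyDamage reduces Health, printing it or destroying Grux at zero.
; Tick keeps its widget facing the camera.
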(event `self.ReceiveTick`
  (params (DeltaSeconds :type "Float (single-precision)"))
  (`|ExecutionSequence`
    (:`then_0`
      (if (not (`self.isSeeingplayer`))
        (`MovementComponent.StopMovementImmediately` (`self.CharacterMovement`))))
    (:`then_1`
      (`SceneComponent.K2_SetWorldRotation` (`self.Widget`) (`KismetMathLibrary.FindLookAtRotation` (`SceneComponent.K2_GetComponentLocation` (`self.Widget`)) (`SceneComponent.K2_GetComponentLocation` (`PlayerCameraManager.TransformComponent` (`GameplayStatics.GetPlayerCameraManager` 0)))) false false))))

(event `self.PawnSensing.OnSeePawn`
  (params (Pawn :type "Pawn Object Reference"))
  ;[1 1 1] Perseguir IA
  (set `self.isSeeingplayer` true)
  (`self.FollowPlayer`))

(event `FollowPlayer`
  ;[1 1 1] Perseguir IA
  (set `self.canAttack` true)
  (if (`self.isSeeingplayer`)
    (`|AIMoveTo` self (0.0 0.0 0.0) (`GameplayStatics.GetPlayerCharacter` 0) 150.0
      (:`OnSuccess`
        (if (`self.canAttack`)
          (set `self.canAttack` false)
          (bind _returnvalue (`self.PlayAnimMontage` "/Game/lasto/animaciones/Gruxattack_Montage.Gruxattack_Montage"))
          (bind _outactors (`KismetSystemLibrary.SphereOverlapActors` (`SceneComponent.K2_GetComponentLocation` (`self.Arrow1`)) 100.0 (`self.Object Types`)))
          (for _array_element _outactors
            (if (`self.ActorHasTag` _array_element "player")
              (`GameplayStatics.ApplyDamage` _array_element 20.0)))
          (`KismetSystemLibrary.Delay` _returnvalue)
          (set `self.canAttack` true))))
    (else
      (set `self.isSeeingplayer` false))))

(event `self.ReceiveAnyDamage`
  (params (Damage :type "Float (single-precision)") (DamageType :type "DamageType Object Reference") (InstigatedBy :type "Controller Object Reference") (DamageCauser :type "Actor Object Reference"))
  ;[1 1 1] Recibir Daño
  (set `self.Health` (- (`self.Health`) Damage))
  (if (<= (`self.Health`) 0.0)
    (`KismetSystemLibrary.PrintString` "Grux dead" true true (struct :`R` 1.0 :`A` 1.0))
    (`self.K2_DestroyActor`)
    (else
      (`KismetSystemLibrary.PrintString` (`KismetStringLibrary.Conv_DoubleToString` (`self.Health`)) true true (struct :`R` 1.0 :`A` 1.0)))))

(fn `UserConstructionScript`)